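; Dark Knight hero character Blueprint, a selectable party member with weapons, skills and an overhead health/resource bar.
; BeginPlay equips main-hand and offhand weapons and passes three skills to the CombatSystem.
; Tick pushes health and resource percentages to the HealthUI widget and billboards it against the camera view, preserving its pitch.
; Selection events toggle the bar's highlight and update the player controller's DungeonHUD utilities and character button.
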(event `self.ReceiveTick`
  (params (DeltaSeconds :type "Float (single-precision)"))
  (`parent.ReceiveTick` DeltaSeconds)
  (bind _ashero_health_bar (cast `/Game/Widgets/HeroHealthBar` (`WidgetComponent.GetWidget` (`self.HealthUI`))))
  (`self.UpdateHealthResourceUI` _ashero_health_bar)
  ;[1 1 1] Rotate UI following camera
  (`self.RotateUI`))

(event `self.ReceiveBeginPlay`
  (`parent.ReceiveBeginPlay`)
  (`self.TryEquipWeapon` (`self.MainHand`) true)
  (`self.TryEquipWeapon` (`self.Offhand`))
  (`MMOCombatSystem.SetSkills` (`self.CombatSystem`) (`|MakeArray` (`self.Skill 1`) (`self.Skill 2`) (`self.Skill 3`))))

(event `self.OnSelected`
  (bind _ashero_health_bar (cast `/Game/Widgets/HeroHealthBar` (`WidgetComponent.GetWidget` (`self.HealthUI`))))
  (`/Game/Widgets/HeroHealthBar.ToggleCharSelection` _ashero_health_bar true)
  (bind _asmmoplayer_controller_bp (cast `/Game/Blueprints/Core/MMOPlayerController_BP` (`GameplayStatics.GetPlayerController` 0)))
  (bind _dungeonhud (`/Game/Blueprints/Core/MMOPlayerController_BP.DungeonHUD` _asmmoplayer_controller_bp))
  (`/Game/Widgets/DungeonUI.ToggleCharUtilities` _dungeonhud true)
  (`/Game/Widgets/DungeonUI.UpdateCharButton` _dungeonhud true self))

(event `self.OnDeselected`
  (bind _ashero_health_bar (cast `/Game/Widgets/HeroHealthBar` (`WidgetComponent.GetWidget` (`self.HealthUI`))))
  (`/Game/Widgets/HeroHealthBar.ToggleCharSelection` _ashero_health_bar false)
  (bind _asmmoplayer_controller_bp (cast `/Game/Blueprints/Core/MMOPlayerController_BP` (`GameplayStatics.GetPlayerController` 0)))
  (bind _dungeonhud (`/Game/Blueprints/Core/MMOPlayerController_BP.DungeonHUD` _asmmoplayer_controller_bp))
  (`/Game/Widgets/DungeonUI.ToggleCharUtilities` _dungeonhud false)
  (`/Game/Widgets/DungeonUI.UpdateCharButton` _dungeonhud false self))

(fn `RotateUI`
  (bind _healthui (`self.HealthUI`))
  (bind (_returnvalue_roll _returnvalue_pitch) (`KismetMathLibrary.BreakRotator` (`SceneComponent.K2_GetComponentRotation` _healthui)))
  (bind (_returnvalue_roll_2 _returnvalue_pitch_2 _returnvalue_yaw) (`KismetMathLibrary.BreakRotator` (`KismetMathLibrary.FindLookAtRotation` (`self.K2_GetActorLocation`) (+ (`self.K2_GetActorLocation`) (* (`KismetMathLibrary.GetForwardVector` (`.Rotation` (`Controller.GetPlayerViewPoint` (`GameplayStatics.GetPlayerController` 0)))) -20000.0)))))
  (`SceneComponent.K2_SetWorldRotation` _healthui (`KismetMathLibrary.MakeRotator` _returnvalue_roll_2 _returnvalue_pitch _returnvalue_yaw) false false))

(fn `UpdateHealthResourceUI`
  (params (HealthUI :type "/Game/Widgets/HeroHealthBar Object Reference"))
  (`/Game/Widgets/HeroHealthBar.SetHealthValue` HealthUI (`self.GetHealthPercent`))
  (`/Game/Widgets/HeroHealthBar.SetManaValue` HealthUI (`self.GetResourcePercent`)))

(fn `UserConstructionScript`)