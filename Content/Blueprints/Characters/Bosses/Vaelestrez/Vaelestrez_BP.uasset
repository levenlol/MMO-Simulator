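; Boss character Blueprint for Vaelestrez, which equips a claw as its main-hand weapon and fights with Bite and Fire Nova skills.
; On BeginPlay it runs the parent setup, attempts the weapon equip and passes both skills to its CombatSystem.
; Heroes entering the AggroSphere are registered with the AggroManager as threats with no extra aggro boost.
; Damage taken spawns floating combat text at the boss's location.
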(event `self.ReceiveBeginPlay`
  (`parent.ReceiveBeginPlay`)
  (`self.TryEquipWeapon` "/Game/Blueprints/Characters/Bosses/Vaelestrez/VaelestrezClaw_BP.VaelestrezClaw_BP_C" true)
  (`MMOCombatSystem.SetSkills` (`self.CombatSystem`) (`|MakeArray` "/Game/Blueprints/Characters/Bosses/Vaelestrez/Vaelestrez_Bite_Skill_BP.Vaelestrez_Bite_Skill_BP_C" "/Game/Blueprints/Characters/Bosses/Vaelestrez/Vaelestrez_FIreNova_Skill_BP.Vaelestrez_FIreNova_Skill_BP_C" :!type "MMOWrapperSkill Class Reference")))

(event `self.AggroSphere.OnComponentBeginOverlap`
  (params (OverlappedComponent :type "PrimitiveComponent Object Reference") (OtherActor :type "Actor Object Reference") (OtherComp :type "PrimitiveComponent Object Reference") (OtherBodyIndex :type Integer) (bFromSweep :type Boolean) (SweepResult :type "HitResult Structure (by ref)"))
  (bind _asmmobase_hero (cast `MMOBaseHero` OtherActor))
  (`MMOAggroManagerComponent.AddDanger` (`self.AggroManager`) _asmmobase_hero 0.0))

(event `self.DamageTake`
  (params (InDamage :type "MMODamage Structure"))
  (`MMOFloatingCombatTextComponent.AddFloatingText` (`self.MMOFloatingCombatText`) InDamage (`self.K2_GetActorLocation`)))

(fn `UserConstructionScript`
  (`parent.UserConstructionScript`))