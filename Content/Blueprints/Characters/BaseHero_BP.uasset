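; Base hero character Blueprint that equips main-hand and offhand weapons and hands three skills to its CombatSystem on begin play.
; Each tick it refreshes health and resource bars, yaws the health widget against camera view, and shows a cast bar for the furthest-progressed casting skill.
; Damage events spawn floating combat text.
; Selection and deselection toggle the health bar highlight and update the player controller's DungeonHUD.
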(event `self.ReceiveTick`
  (params (DeltaSeconds :type "Float (single-precision)"))
  (`parent.ReceiveTick` DeltaSeconds)
  (bind _ashero_health_bar (cast `/Game/Widgets/HeroHealthBar` (`WidgetComponent.GetWidget` (`self.HealthUI`))))
  (`self.UpdateHealthResourceUI` _ashero_health_bar)
  ;[1 1 1] Rotate UI following camera
  (`self.RotateUI`)
  (`self.UpdateCastBar`))

(event `self.ReceiveBeginPlay`
  (`parent.ReceiveBeginPlay`)
  (add `self.OnDamageTaken` (delegate `OnDamageTaken_Event`))
  (`self.TryEquipWeapon` (`self.MainHand`) true)
  (`self.TryEquipWeapon` (`self.Offhand`))
  (`MMOCombatSystem.SetSkills` (`self.CombatSystem`) (`|MakeArray` (`self.Skill 1`) (`self.Skill 2`) (`self.Skill 3`))))

(event `OnDamageTaken_Event` :!signature `self.OnDamageTaken`
  (params (Sender :type "MMOBaseCharacter Object Reference") (Damage :type "MMODamage Structure"))
  (`MMOFloatingCombatTextComponent.AddFloatingText` (`self.MMOFloatingCombatText`) Damage (`self.K2_GetActorLocation`)))

(event `self.OnSelected`
  (bind _ashero_health_bar (cast `/Game/Widgets/HeroHealthBar` (`WidgetComponent.GetWidget` (`self.HealthUI`))))
  (`/Game/Widgets/HeroHealthBar.ToggleCharSelection` _ashero_health_bar true)
  (bind _asmmoplayer_controller_bp (cast `/Game/Blueprints/Core/MMOPlayerController_BP` (`GameplayStatics.GetPlayerController` 0)))
  (bind _dungeonhud (`/Game/Blueprints/Core/MMOPlayerController_BP.DungeonHUD` _asmmoplayer_controller_bp))
  (`/Game/Widgets/DungeonUI.ToggleCharUtilities` _dungeonhud true)
  (`/Game/Widgets/DungeonUI.UpdateCharButton` _dungeonhud true self))

(event `self.OnDeselected`
  (bind _ashero_health_bar (cast `/Game/Widgets/HeroHealthBar` (`WidgetComponent.GetWidget` (`self.HealthUI`))))
  (`/Game/Widgets/HeroHealthBar.ToggleCharSelection` _ashero_health_bar false)
  (bind _asmmoplayer_controller_bp (cast `/Game/Blueprints/Core/MMOPlayerController_BP` (`GameplayStatics.GetPlayerController` 0)))
  (bind _dungeonhud (`/Game/Blueprints/Core/MMOPlayerController_BP.DungeonHUD` _asmmoplayer_controller_bp))
  (`/Game/Widgets/DungeonUI.ToggleCharUtilities` _dungeonhud false)
  (`/Game/Widgets/DungeonUI.UpdateCharButton` _dungeonhud false self))

(fn `RotateUI`
  (bind _healthui (`self.HealthUI`))
  (bind (_returnvalue_roll _returnvalue_pitch) (`KismetMathLibrary.BreakRotator` (`SceneComponent.K2_GetComponentRotation` _healthui)))
  (bind (_returnvalue_roll_2 _returnvalue_pitch_2 _returnvalue_yaw) (`KismetMathLibrary.BreakRotator` (`KismetMathLibrary.FindLookAtRotation` (`self.K2_GetActorLocation`) (+ (`self.K2_GetActorLocation`) (* (`KismetMathLibrary.GetForwardVector` (`.Rotation` (`Controller.GetPlayerViewPoint` (`GameplayStatics.GetPlayerController` 0)))) -20000.0)))))
  (`SceneComponent.K2_SetWorldRotation` _healthui (`KismetMathLibrary.MakeRotator` _returnvalue_roll_2 _returnvalue_pitch _returnvalue_yaw) false false))

(fn `UpdateCastBar`
  (locals (MaxPercent :type "Float (double-precision)"))
  (bind _castbar (`self.CastBar`))
  (bind _ascast_bar_w (cast `/Game/Widgets/CastBar_W` (`WidgetComponent.GetWidget` (`self.CastBar`))))
  (set `local.MaxPercent` 0.0)
  (for _array_element (`MMOCombatSystem.Skills` (`self.CombatSystem`))
    (if (`MMOWrapperSkill.IsCasting` _array_element)
      (set `local.MaxPercent` (`KismetMathLibrary.FMax` (`MMOWrapperSkill.GetCastingPercent` _array_element) (`local.MaxPercent`)))))
  (if (> (`local.MaxPercent`) 0.0)
    (`SceneComponent.SetVisibility` _castbar true false)
    (`/Game/Widgets/CastBar_W.SetProgressBarPercentage` _ascast_bar_w (`local.MaxPercent`))
    (else
      (`SceneComponent.SetVisibility` _castbar false false))))

(fn `UpdateHealthResourceUI`
  (params (HealthUI :type "/Game/Widgets/HeroHealthBar Object Reference"))
  (`/Game/Widgets/HeroHealthBar.SetHealthValue` HealthUI (`self.GetHealthPercent`))
  (`/Game/Widgets/HeroHealthBar.SetManaValue` HealthUI (`self.GetResourcePercent`)))

(fn `UserConstructionScript`)