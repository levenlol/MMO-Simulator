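; BaseEnemy_BP is an enemy character Blueprint with a health and mana bar widget and a debug waypoint patrol.
; On BeginPlay and whenever damage is taken, it pushes health and resource percentages to the EnemyHealthBar widget.
; Each tick, DebugMoveBetweenPoints uses SimpleMoveToActor toward the current waypoint, advancing the index within 150 units and wrapping it to loop the route.
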(event `self.ReceiveBeginPlay`
  (`parent.ReceiveBeginPlay`)
  (add `self.OnDamageTaken` (delegate `OnDamageTaken_Event`))
  (bind _asenemy_health_bar (cast `/Game/Widgets/EnemyHealthBar` (`WidgetComponent.GetWidget` (`self.Healthbar`)) :!label _label))
  (`/Game/Widgets/EnemyHealthBar.SetHealthValue` _asenemy_health_bar (`self.GetHealthPercent`))
  (`/Game/Widgets/EnemyHealthBar.SetManaValue` _asenemy_health_bar (`self.GetResourcePercent`)))

(event `OnDamageTaken_Event` :!signature `self.OnDamageTaken`
  (params (Sender :type "MMOBaseCharacter Object Reference") (Damage :type "MMODamage Structure"))
  (goto _label))

(event `self.ReceiveTick`
  (params (DeltaSeconds :type "Float (single-precision)"))
  (`parent.ReceiveTick` DeltaSeconds)
  (`self.DebugMoveBetweenPoints`))

(fn `UserConstructionScript`)