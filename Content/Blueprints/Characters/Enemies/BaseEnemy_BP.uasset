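; Base enemy character Blueprint that equips weapons, shows a floating health bar and tracks hero aggro.
; On BeginPlay it equips its main and off-hand weapon classes, then fills the EnemyHealthBar widget with health and resource percentages, refreshing it whenever damage is taken.
; Heroes entering the AggroSphere are registered with the AggroManager as threats.
; On death it destroys both held weapons and then itself.
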(event `self.ReceiveBeginPlay`
  (`parent.ReceiveBeginPlay`)
  (`self.TryEquipWeapon` (`self.MainHand`) true)
  (`self.TryEquipWeapon` (`self.OffHand`))
  (add `self.OnDamageTaken` (delegate `OnDamageTaken_Event`))
  (bind _asenemy_health_bar (cast `/Game/Widgets/EnemyHealthBar` (`WidgetComponent.GetWidget` (`self.Healthbar`)) :!label _label))
  (`/Game/Widgets/EnemyHealthBar.SetHealthValue` _asenemy_health_bar (`self.GetHealthPercent`))
  (`/Game/Widgets/EnemyHealthBar.SetManaValue` _asenemy_health_bar (`self.GetResourcePercent`)))

(event `OnDamageTaken_Event` :!signature `self.OnDamageTaken`
  (params (Sender :type "MMOBaseCharacter Object Reference") (Damage :type "MMODamage Structure"))
  (goto _label))

(event `self.ReceiveTick`
  (params (DeltaSeconds :type "Float (single-precision)"))
  (`parent.ReceiveTick` DeltaSeconds))

(event `self.AggroSphere.OnComponentBeginOverlap`
  (params (OverlappedComponent :type "PrimitiveComponent Object Reference") (OtherActor :type "Actor Object Reference") (OtherComp :type "PrimitiveComponent Object Reference") (OtherBodyIndex :type Integer) (bFromSweep :type Boolean) (SweepResult :type "HitResult Structure (by ref)"))
  (bind _asmmobase_hero (cast `MMOBaseHero` OtherActor))
  (`MMOAggroManagerComponent.AddDanger` (`self.AggroManager`) _asmmobase_hero 0.0))

(event `self.Die`
  (bind _returnvalue (`self.GetMainHandWeapon`))
  (bind _returnvalue_2 (`self.GetOffHandWeapon`))
  ;[1 1 1] Die
  (`/Engine/EditorBlueprintResources/StandardMacros.IsValid` _returnvalue
    (:`Is Valid`
      (`self.K2_DestroyActor` _returnvalue))
    (:`Is Not Valid`
      _))
  (`/Engine/EditorBlueprintResources/StandardMacros.IsValid` _returnvalue_2
    (:`Is Valid`
      (`self.K2_DestroyActor` _returnvalue_2))
    (:`Is Not Valid`
      _))
  (`self.K2_DestroyActor` self))

(fn `UserConstructionScript`)